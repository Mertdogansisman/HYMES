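; BP_Enemy is an enemy actor that turns to face the player within range and fires bullets on a looping timer, regardless of range.
; Short-Delay recursive events, rather than Tick, check distance and snap yaw with a -90 degree offset.
; Fire spawns BP_EnemyBullet at ShootingPoint.
; AnyDamage reduces clamped health without triggering death, and an F key handler calls ApplyDamage on the player with no amount set.
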(event Custom|Fire
  (bind _shooting_point (Variables|Default|GetShooting%20Point))
  (Game|SpawnActorfromClass "/Game/Blueprints/Enemy/BP_EnemyBullet.BP_EnemyBullet_C" (Math|Transform|MakeTransform (.Location (Math|Transform|BreakTransform (Transformation|GetWorldTransform (Variables|Default|GetShooting%20Point)))) (Math|Rotator|MakeRotfromXY (Math|Vector|GetRightVector _shooting_point) (Math|Vector|GetForwardVector _shooting_point)) "1.000000,1.000000,1.000000") "Undefined" "MultiplyWithRoot" 0 0))

(event Custom|Should%20Rotate%20Event
  ;[1 1 1] Check should rotate
  (if (<= (Transformation|GetDistanceTo (Variables|Default|GetChar%20REF)) 9e+02)
    (Variables|Default|SetShould%20Rotate%20? true)
    (CallFunction|FacePlayer)
    (else
      (Variables|Default|SetShould%20Rotate%20? false)))
  (Utilities|FlowControl|Delay 0.001)
  (CallFunction|ShouldRotateEvent))

(event Custom|Face%20Player
  ;[1 1 1] Always Face Player
  (if (Variables|Default|GetShould%20Rotate%20?)
    (Transformation|SetActorRotation (Math|Rotator|MakeRotator 0.0 0.0 (+ (.Yaw (Math|Rotator|BreakRotator (Math|Rotator|FindLookatRotation (Transformation|GetActorLocation self) (Transformation|GetActorLocation (Game|GetPlayerCharacter 0))))) -9e+01)))
    (Utilities|FlowControl|Delay 0.001)
    (CallFunction|FacePlayer)
    (else
      (CallFunction|ShouldRotateEvent))))

(event EventBeginPlay
  (Utilities|FlowControl|Sequence
    (:then_0
      (Utilities|Time|SetTimerbyEvent (delegate Custom|Fire) (Variables|Shooting|GetFireRate) true))
    (:then_1
      (bind _asbp_third_person_character (Utilities|Casting|CastToBP_ThirdPersonCharacter (Game|GetPlayerCharacter 0)))
      (Variables|Default|SetChar%20REF _asbp_third_person_character)
      (CallFunction|ShouldRotateEvent))))

(event EventTick
  (params (DeltaSeconds :type Float%20%28single-precision%29)))

(event Game|Damage|EventAnyDamage
  (params (Damage :type Float%20%28single-precision%29) (DamageType :type Damage%20Type%20Object%20Reference) (InstigatedBy :type Controller%20Object%20Reference) (DamageCauser :type Actor%20Object%20Reference))
  ;[1 1 1] Health system
  (if (not (Variables|Default|GetIs%20Dead))
    (Variables|Default|SetCurrentHealth (Math|Float|Clamp(Float) (- (Variables|Default|GetCurrentHealth) Damage) 0.0 (Variables|Default|GetMaxHealth)))))

(event Input|KeyboardEvents|F
  (params (Key :type Key%20Structure :default "None"))
  (:Pressed
    (Game|Damage|ApplyDamage (Variables|Default|GetChar%20REF) 0.0 0 0)))

(fn ConstructionScript)